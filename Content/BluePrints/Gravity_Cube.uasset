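; Physics cube whose gravity flips upward while the GrappleCharacter overlaps a GravityTrigger1_Blueprint, and downward otherwise.
; BeginPlay caches the last-found character and trigger.
; Tick adds GravVelocity to the cube's linear velocity each frame, without delta-time scaling, then resets it from the overlap test.
; The G key also flip-flops GravVelocity, but Tick overwrites that value; a MultiGate alternative is unconnected.
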(event EventBeginPlay
  (bind _outactors (Actor|GetAllActorsOfClass "/Game/FirstPersonBP/Blueprints/GrappleCharacter.GrappleCharacter_C"))
  (for _array_element _outactors
    (Variables|Default|SetGrappleCharacter _array_element)
    (bind _outactors_2 (Actor|GetAllActorsOfClass "/Game/GravityTrigger1_Blueprint.GravityTrigger1_Blueprint_C"))
    (for _array_element_2 _outactors_2
      (Variables|Default|SetTriggerbox _array_element_2))))

(event EventTick
  (params (DeltaSeconds :type Float%20%28single-precision%29))
  (bind _returnvalue (Physics|GetPhysicsLinearVelocity (Variables|Default|GetCube) "None"))
  (Physics|SetPhysicsLinearVelocity (Variables|Default|GetCube) (+ _returnvalue (Variables|Default|GetGravVelocity)) false "None")
  (if (Collision|IsOverlappingActor (Variables|Default|GetTriggerbox) (Variables|Default|GetGrappleCharacter) :!class /Script/Engine.Actor)
    (Variables|Default|SetGravVelocity "0.000000, 0,20.000000")
    (else
      (Variables|Default|SetGravVelocity "0, 0,-20.000000"))))

(event Input|KeyboardEvents|G
  (params (Key :type Key%20Structure))
  (:Pressed
    (Utilities|FlowControl|FlipFlop
      (:A
        (Variables|Default|SetGravVelocity "0, 0,20.000000"))
      (:B
        (Variables|Default|SetGravVelocity "0, 0,-20.000000")))))

(fn ConstructionScript)