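; Crane actor Blueprint that the player controls by keyboard, enabling input from player controller 0 on BeginPlay.
; Z and X turn the root component in quarter-turn yaw steps, while C and V raise and lower the Hook in fixed world-space steps.
; Tick also adds the Rotation variable as yaw every frame without delta-time scaling, and applies a zero offset to the Hook, leaving it in place.
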(event EventBeginPlay
  (Input|EnableInput (Game|GetPlayerController 0)))

(event EventTick
  (params (DeltaSeconds :type Float%20%28single-precision%29))
  (bind _hook (Variables|Default|GetHook))
  (Transformation|AddWorldRotation (Variables|Default|GetDefaultSceneRoot) (Math|Rotator|MakeRotator 0.0 0.0 (Variables|Default|GetRotation)) false false)
  (Transformation|SetWorldLocation _hook (+ (Transformation|GetWorldLocation _hook) (Math|Vector|MakeVector 0.0 0.0 0.0)) false false))

(event Input|KeyboardEvents|Z
  (params (Key :type Key%20Structure :default "AnyKey"))
  ;[1 1 1] R Left
  (:Pressed
    (Transformation|AddWorldRotation (Variables|Default|GetDefaultSceneRoot) "0.000000,90.000000,0.000000" false false)))

(event Input|KeyboardEvents|X
  (params (Key :type Key%20Structure :default "AnyKey"))
  ;[1 1 1] R Right
  (:Pressed
    (Transformation|AddWorldRotation (Variables|Default|GetDefaultSceneRoot) "0.000000,-90.000000,0.000000" false false)))

(event Input|KeyboardEvents|C
  (params (Key :type Key%20Structure :default "AnyKey"))
  (bind _hook (Variables|Default|GetHook))
  ;[1 1 1] Hook U
  (:Pressed
    (Transformation|SetWorldLocation _hook (+ (Transformation|GetWorldLocation _hook) "0, 0,30.000000") false false)))

(event Input|KeyboardEvents|V
  (params (Key :type Key%20Structure :default "AnyKey"))
  (bind _hook (Variables|Default|GetHook))
  ;[1 1 1] Hook D
  (:Pressed
    (Transformation|SetWorldLocation _hook (+ (Transformation|GetWorldLocation _hook) "0, 0,-30.000000") false false)))

(fn ConstructionScript)