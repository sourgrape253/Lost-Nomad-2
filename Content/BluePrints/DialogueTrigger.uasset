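; DialogueTrigger is an overlap trigger that plays a scripted intro voice sequence, with lines about hull failure, suit damage, planet scanning and ship systems.
; On the first actor overlap, a DoOnce gate fires a HeadTruama camera shake on the player camera.
; A fixed chain of Delay nodes then spawns each 2D dialogue sound in turn, with hand-timed gaps and no check on the overlapping actor.
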(event Collision|EventActorBeginOverlap
  (params (OtherActor :type Actor%20Object%20Reference))
  (Utilities|FlowControl|DoOnce false
    (:Completed
      (Class|PlayerCameraManager|PlayCameraShake (Game|GetPlayerCameraManager 0) "/Game/HeadTruama.HeadTruama_C" 1.0 "CameraLocal" "0, 0, 0")
      (Utilities|FlowControl|Delay 0.5)
      (Audio|SpawnSound2D "/Game/Audio/Character/Suit/1_hello.1_hello")
      (Utilities|FlowControl|Delay 3.5)
      (Audio|SpawnSound2D "/Game/Audio/Character/Suit/2_hullFailure.2_hullFailure")
      (Utilities|FlowControl|Delay 5.0)
      (Audio|SpawnSound2D "/Game/Audio/Character/Suit/9_scanningPlanet.9_scanningPlanet")
      (Utilities|FlowControl|Delay 2.5)
      (Audio|SpawnSound2D "/Game/Audio/Character/Suit/10_planetGravity.10_planetGravity")
      (Utilities|FlowControl|Delay 4.5)
      (Audio|SpawnSound2D "/Game/Audio/Character/Suit/3_distanceEarth.3_distanceEarth")
      (Utilities|FlowControl|Delay 3.5)
      (Audio|SpawnSound2D "/Game/Audio/Character/Suit/4_suitDamage.4_suitDamage")
      (Utilities|FlowControl|Delay 3.0)
      (Audio|SpawnSound2D "/Game/Audio/Character/Suit/5_thrustersOnline.5_thrustersOnline")
      (Utilities|FlowControl|Delay 1.5)
      (Audio|SpawnSound2D "/Game/Audio/Character/Suit/6_powerjumpOnline.6_powerjumpOnline")
      (Utilities|FlowControl|Delay 1.5)
      (Audio|SpawnSound2D "/Game/Audio/Character/Suit/7_landingGear.7_landingGear")
      (Utilities|FlowControl|Delay 2.0)
      (Audio|SpawnSound2D "/Game/Audio/Character/Suit/8_seekAssistance.8_seekAssistance")
      (Utilities|FlowControl|Delay 4.5)
      (Audio|SpawnSound2D "/Game/Audio/Character/Suit/11_oddsSurvival.11_oddsSurvival"))))

(fn ConstructionScript)